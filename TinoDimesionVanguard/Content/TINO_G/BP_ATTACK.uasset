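; Attack component for TINO_G_BP that runs a three-hit melee combo from the IA_ATTACK input.
; Each press briefly shows both weapons and plays the current combo montage; montage notifies reopen input and advance the counter, which a timer resets.
; StartAttackTrace schedules a very wide sphere overlap at the right weapon that damages Enemy-tagged actors, and StopAttackTrace clears that timer.
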(event Custom|Reset%20COunter
  (Variables|Default|SetComboCoounter 0))

(event Custom|Hidden
  (Rendering|SetVisibility (Variables|Default|GetLeft%20Weapon) false false))

(event Custom|Start%20AttackTrace
  (bind _returnvalue (Utilities|Time|SetTimerbyEvent (delegate Custom|Attack%20Trace) 0.01))
  (Variables|Default|SetAttack%20Timer%20H _returnvalue))

(event Custom|Attack%20Trace
  (bind _outactors (Collision|SphereOverlapActors (Transformation|GetWorldLocation (Variables|Default|GetRight%20Weapon)) 1e+04 (Variables|Default|GetObject%20Types) 0))
  (if true
    (bind _array_element (Utilities|Array|ForEachLoopwithBreak _outactors)
      (:LoopBody
        (if (Actor|ActorHasTag _array_element "Enemy")
          (Game|Damage|ApplyDamage _array_element 2e+01 0 0)))
      (:Completed
        (Development|PrintText "Attack?")))))

(event Custom|StopAttackTrace
  (Utilities|Time|ClearandInvalidateTimerbyHandle (Variables|Default|GetAttack%20Timer%20H)))

(event Input|EnhancedActionEvents|EnhancedInputActionIA_ATTACK
  (params (ActionValue :type Boolean) (ElapsedSeconds :type Float%20%28double-precision%29) (TriggeredSeconds :type Float%20%28double-precision%29) (InputAction :type Input%20Action%20Object%20Reference :default "/Game/TINO_G/IA_TINO/IA_ATTACK.IA_ATTACK"))
  (bind _mesh (Variables|Default|GetMesh))
  (:Started
    (if (not (Variables|Default|GetIs%20Attack?))
      (Variables|Default|SetIs%20Attack? true)
      (Rendering|SetVisibility (Variables|Default|GetLeft%20Weapon) true false)
      (Utilities|Time|SetTimerbyEvent (delegate Custom|Hidden) 5.0)
      (switch int (Variables|Default|GetComboCoounter)
        (:0
          (Animation|Montage|PlayMontage _mesh "/Game/TINO_G/TINO_ANI/Attack_1_Montage.Attack_1_Montage"
            (:then
              (Utilities|Time|SetTimerbyEvent (delegate Custom|Reset%20COunter) 1.0 :!label _label))
            (:OnNotifyBegin
              (Variables|Default|SetIS%20Attack? false)
              (Variables|Default|SetComboCoounter 1))))
        (:1
          (Animation|Montage|PlayMontage _mesh "/Game/TINO_G/TINO_ANI/Attack_2_Montage.Attack_2_Montage"
            (:then
              (goto _label))
            (:OnNotifyBegin
              (Variables|Default|SetIS%20Attack? false)
              (Variables|Default|SetComboCoounter 2))))
        (:2
          (Animation|Montage|PlayMontage _mesh "/Game/TINO_G/TINO_ANI/Attack_3_Montage.Attack_3_Montage"
            (:then
              (goto _label))
            (:OnNotifyBegin
              (Variables|Default|SetIS%20Attack? false)
              (Variables|Default|SetComboCoounter 0))))))))

(event EventBeginPlay
  (bind _astino_g_bp (Utilities|Casting|CastToTINO_G_BP (Components|GetOwner)))
  (bind _output_get (Variables|Default|SetTINO%20G _astino_g_bp))
  (Variables|Default|SetMesh (Variables|/Script/Engine.Character|GetMesh _output_get))
  (Variables|Default|SetLeft%20Weapon (Variables|/Game/TINO_G/TINO_G_BP.TINO_G_BP_C|GetLeft%20Weapon _astino_g_bp))
  (Variables|Default|SetRight%20Weapon (Variables|/Game/TINO_G/TINO_G_BP.TINO_G_BP_C|GetRight%20Weapon _astino_g_bp)))