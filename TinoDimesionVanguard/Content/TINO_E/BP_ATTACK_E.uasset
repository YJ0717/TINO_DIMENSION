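; Attack component for TINO_E_BP that handles rifle shots with a three-step montage combo on IA_ATTACK input.
; Each accepted press spawns a BP_Bullet along the RiffleC forward vector, alongside a debug line trace whose result is unused.
; It also shows the right weapon temporarily and plays the current combo montage.
; A montage notify unlocks the next attack and advances the combo, while a short timer resets the counter.
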(event Custom|Reset%20COunter
  (Variables|Default|SetComboCT 0))

(event Custom|Hidden
  (Rendering|SetVisibility (Variables|Default|GetRight%20Weapon) false false))

(event Custom|Riffle%20At
  (bind _tino_e (Variables|Default|GetTINO%20E))
  (bind _riffle_c (Variables|/Game/TINO_E/TINO_E_BP.TINO_E_BP_C|GetRiffle%20C _tino_e))
  (bind _returnvalue (Transformation|GetWorldLocation _riffle_c))
  (bind _returnvalue_2 (Math|Vector|GetForwardVector _riffle_c))
  (bind _returnvalue_3 (* _returnvalue_2 2e+04))
  (bind _returnvalue_4 (+ _returnvalue _returnvalue_3))
  (Collision|LineTraceByChannel _returnvalue _returnvalue_4 "TraceTypeQuery1" false 0 "ForDuration")
  (Game|SpawnActorfromClass "/Game/TINO_E/TINO_E_Weapon/BP_Bullet.BP_Bullet_C" (Math|Transform|MakeTransform _returnvalue (Math|Rotator|FindLookatRotation _returnvalue _returnvalue_4)) "Undefined" "MultiplyWithRoot" 0 0))

(event Input|EnhancedActionEvents|EnhancedInputActionIA_ATTACK
  (params (ActionValue :type Boolean) (ElapsedSeconds :type Float%20%28double-precision%29) (TriggeredSeconds :type Float%20%28double-precision%29) (InputAction :type Input%20Action%20Object%20Reference :default "/Game/TINO_G/IA_TINO/IA_ATTACK.IA_ATTACK"))
  (bind _mesh (Variables|Default|GetMesh))
  (:Started
    (if (not (Variables|Default|GetAttack?))
      (CallFunction|Riffleat)
      (Variables|Default|SetAttack? true)
      (Rendering|SetVisibility (Variables|Default|GetRight%20Weapon) true false)
      (Utilities|Time|SetTimerbyEvent (delegate Custom|Hidden) 5.0)
      (switch int (Variables|Default|GetComboCT)
        (:0
          (Animation|Montage|PlayMontage _mesh "/Game/TINO_E/TINO_E_ANI/Attack_1_Montage.Attack_1_Montage"
            (:then
              (Utilities|Time|SetTimerbyEvent (delegate Custom|Reset%20COunter) 1.0 :!label _label))
            (:OnNotifyBegin
              (Variables|Default|SetAttack? false)
              (Variables|Default|SetComboCT 1))))
        (:1
          (Animation|Montage|PlayMontage _mesh "/Game/TINO_E/TINO_E_ANI/Attack_2_Montage.Attack_2_Montage"
            (:then
              (goto _label))
            (:OnNotifyBegin
              (Variables|Default|SetAttack? false)
              (Variables|Default|SetComboCT 2))))
        (:2
          (Animation|Montage|PlayMontage _mesh "/Game/TINO_E/TINO_E_ANI/Attack_3_Montage.Attack_3_Montage"
            (:then
              (goto _label))
            (:OnNotifyBegin
              (Variables|Default|SetAttack? false)
              (Variables|Default|SetComboCT 0))))))))

(event EventBeginPlay
  (bind _astino_e_bp (Utilities|Casting|CastToTINO_E_BP (Components|GetOwner)))
  (bind _output_get (Variables|Default|SetTINO%20E _astino_e_bp))
  (Variables|Default|SetMesh (Variables|/Script/Engine.Character|GetMesh _output_get))
  (Variables|Default|SetRight%20Weapon (Variables|/Game/TINO_E/TINO_E_BP.TINO_E_BP_C|GetRight%20Weapon _astino_e_bp)))