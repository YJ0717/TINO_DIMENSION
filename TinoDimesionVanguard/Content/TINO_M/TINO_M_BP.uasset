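; Player character Blueprint for TINO that toggles between 3D and 2D cameras, with dash, jump and platform spawning.
; In 2D, a trace from the 2D camera records hit actors' positions in StructArray and snaps static meshes onto the player's X depth.
; Returning to 3D teleports recorded actors back and clears the array.
; STBAR drains in 2D, forcing 3D at zero, and refills in 3D, where look input works.
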(event Input|EnhancedActionEvents|EnhancedInputActionIA_JUMP_TINO
  (params (ActionValue :type Boolean) (ElapsedSeconds :type Float%20%28double-precision%29) (TriggeredSeconds :type Float%20%28double-precision%29) (InputAction :type Input%20Action%20Object%20Reference :default "/Game/TINO_G/IA_TINO/IA_JUMP_TINO.IA_JUMP_TINO"))
  (:Started
    (Character|Jump)))

(event Input|EnhancedActionEvents|EnhancedInputActionIA_ROTATE_TINO
  (params (ActionValue :type Vector%202D%20Structure) (ElapsedSeconds :type Float%20%28double-precision%29) (TriggeredSeconds :type Float%20%28double-precision%29) (InputAction :type Input%20Action%20Object%20Reference :default "/Game/TINO_G/IA_TINO/IA_ROTATE_TINO.IA_ROTATE_TINO"))
  (if (not (stale Input|EnhancedActionEvents|EnhancedInputActionIA_2dCmara _output_get))
    (Pawn|Input|AddControllerYawInput (.x ActionValue))
    (Pawn|Input|AddControllerPitchInput (.y ActionValue))))

(event Input|EnhancedActionEvents|EnhancedInputActionIA_2dCmara
  (params (ActionValue :type Boolean) (ElapsedSeconds :type Float%20%28double-precision%29) (TriggeredSeconds :type Float%20%28double-precision%29) (InputAction :type Input%20Action%20Object%20Reference :default "/Game/TINO_G/2dcamera/IA_2dCmara.IA_2dCmara"))
  (bind _returnvalue (Game|GetPlayerController 0))
  (:Started
    (Utilities|FlowControl|FlipFlop
      (:A
        (bind _output_get (Variables|Default|SetIS_2Dmode? false))
        (Game|Player|SetViewTargetwithBlend _returnvalue (Variables|/Script/Engine.ChildActorComponent|GetChildActor (Variables|Default|Get3dC)) 0.0 "VTBlend_Linear" 0.0 false))
      (:B
        (Variables|Default|SetIS_2Dmode? true)
        (Game|Player|SetViewTargetwithBlend _returnvalue (Variables|/Script/Engine.ChildActorComponent|GetChildActor (Variables|Default|Get2dC)) 0.0 "VTBlend_Linear" 0.0 false)))))

(event EventBeginPlay
  (bind _returnvalue (UserInterface|CreateWidget "/Game/TINO_G/TINO_G_UI.TINO_G_UI_C" (Game|GetPlayerController 0)))
  (UserInterface|Viewport|AddtoViewport _returnvalue 0)
  (Transformation|SetWorldRotation (Variables|Components|GetArrow1) (Pawn|GetControlRotation :!class /Script/Engine.Pawn) false false)
  (Game|Player|SetViewTargetwithBlend (Game|GetPlayerController 0) (Variables|/Script/Engine.ChildActorComponent|GetChildActor (Variables|Default|Get3dC)) 0.0 "VTBlend_Linear" 0.0 false))

(event EventTick
  (params (DeltaSeconds :type Float%20%28single-precision%29))
  (bind _2dc (Variables|Default|Get2dC))
  (bind _returnvalue (Transformation|GetWorldLocation _2dc))
  (Variables|Default|SetSpeed (Math|Vector|VectorLengthXY (Variables|/Script/Engine.MovementComponent|GetVelocity (Variables|Character|GetCharacterMovement))))
  (Utilities|FlowControl|Sequence
    (:then_0
      (if (Variables|Default|GetIS_2Dmode?)
        (bind _outhit (Collision|LineTraceByChannel _returnvalue (+ _returnvalue (* (Math|Vector|GetForwardVector _2dc) 1.5e+03)) "TraceTypeQuery1" false 0 "ForDuration"))
        (Utilities|FlowControl|Sequence
          (:then_0
            (if (.bBlockingHit (Collision|BreakHitResult _outhit))
              (Utilities|FlowControl|DoOnce false :!label _label
                (:Completed
                  (Development|PrintString "do once 실행")
                  (bind _output_get (Variables|Default|Sethit? true))
                  (Development|PrintString (Utilities|String|ToString(Boolean) _output_get))
                  (Variables|Default|SetIs_Move? true)
                  (Utilities|Array|Add (Variables|Default|GetStructArray) (Utilities|Struct|MakeDimesion_Info (.HitActor (Collision|BreakHitResult _outhit)) (Math|Vector|MakeVector (.x (Transformation|GetActorLocation (.HitActor (Collision|BreakHitResult _outhit)))) (.y (Transformation|GetActorLocation (.HitActor (Collision|BreakHitResult _outhit)))) (.z (Transformation|GetActorLocation (.HitActor (Collision|BreakHitResult _outhit)))))))))))
          (:then_1
            (if (.bBlockingHit (Collision|BreakHitResult _outhit))
              (bind _asstatic_mesh_actor (Utilities|Casting|CastToStaticMeshActor (.HitActor (Collision|BreakHitResult _outhit))))
              (bind _output_get_2 (Variables|Default|SetAs%20Static%20Mesh%20Actor _asstatic_mesh_actor))
              (for _array_element (Variables|Default|GetStructArray)
                (if (== (.actor _array_element) (.HitActor (Collision|BreakHitResult _outhit)))
                  (Variables|Default|SetIs_Move? true)
                  (else
                    (Variables|Default|SetIs_Move? false))))
              (if (Variables|Default|GetIs_Move?)
                (Transformation|Teleport _output_get_2 (Math|Vector|MakeVector (.x (Transformation|GetActorLocation (Game|GetPlayerCharacter 0))) (.y (Transformation|GetActorLocation (.HitActor (Collision|BreakHitResult _outhit)))) (.z (Transformation|GetActorLocation (.HitActor (Collision|BreakHitResult _outhit))))) "0, 0, 0")
                (else
                  (Utilities|Array|Add (Variables|Default|GetStructArray) (Utilities|Struct|MakeDimesion_Info (.HitActor (Collision|BreakHitResult _outhit)) (Math|Vector|MakeVector (.x (Transformation|GetActorLocation (.HitActor (Collision|BreakHitResult _outhit)))) (.y (Transformation|GetActorLocation (.HitActor (Collision|BreakHitResult _outhit)))) (.z (Transformation|GetActorLocation (.HitActor (Collision|BreakHitResult _outhit))))))))))))
        (elif (Variables|Default|Gethit?)
          (for _array_element_2 (Variables|Default|GetStructArray)
            (Transformation|Teleport (.actor _array_element_2) (Math|Vector|MakeVector (.x (.object_info _array_element_2)) (.y (.object_info _array_element_2)) (.z (.object_info _array_element_2))) "0, 0, 0")
            (Development|PrintString (Utilities|GetDisplayName (.actor _array_element_2)))
            (Development|PrintString (Utilities|String|ToString(Vector) (Math|Vector|MakeVector (.x (.object_info _array_element_2)) (.y (.object_info _array_element_2)) (.z (.object_info _array_element_2)))))
            (Development|PrintString "돌아감!"))
          (Development|PrintString "원위치")
          (Utilities|Array|Clear (Variables|Default|GetStructArray))
          (bind _output_get_3 (Variables|Default|Sethit? false))
          (Development|PrintString (Utilities|String|ToString(Boolean) _output_get_3))
          (goto _label Reset))))
    (:then_1
      (if (== (Variables|Default|GetST_BAR) 0.0)
        (Variables|Default|SetIS_2Dmode? false)
        (Game|Player|SetViewTargetwithBlend (Game|GetPlayerController 0) (Variables|/Script/Engine.ChildActorComponent|GetChildActor (Variables|Default|Get3dC)) 0.0 "VTBlend_Linear" 0.0 false)))
    (:then_2
      (if (Variables|Default|GetIS_2Dmode?)
        (Utilities|FlowControl|Delay 0.5)
        (Variables|Default|SetST_BAR (Math|Float|Clamp(Float) (- (Variables|Default|GetST_BAR) 0.05)))
        (else
          (Utilities|FlowControl|Delay 0.2)
          (Variables|Default|SetST_BAR (+ (Variables|Default|GetST_BAR) 0.01)))))))

(event Input|KeyboardEvents|Tab
  (params (Key :type Key%20Structure :default "None"))
  (:Pressed
    (for _array_element (Variables|Default|GetStructArray)
      (Development|PrintString (Utilities|GetDisplayName (.actor _array_element)))
      (Development|PrintString (Utilities|String|ToString(Vector) (.object_info _array_element))))))

(event Input|KeyboardEvents|LeftShift
  (params (Key :type Key%20Structure :default "None"))
  (:Pressed
    (Variables|Default|SetDash? true)
    (Variables|/Script/Engine.CharacterMovementComponent|SetMaxWalkSpeed (Variables|Character|GetCharacterMovement) 6e+02))
  (:Released
    (Variables|Default|SetDash? false)
    (Variables|/Script/Engine.CharacterMovementComponent|SetMaxWalkSpeed (Variables|Character|GetCharacterMovement) 3e+02)))

(event Input|KeyboardEvents|U
  (params (Key :type Key%20Structure :default "None"))
  (:Pressed
    (CallFunction|SpawnPlatform)))

(fn ConstructionScript)

(fn SpawnPlatform
  (Game|SpawnActorfromClass "/Game/TINO_M/BP_PLATFORM.BP_PLATFORM_C" (Math|Transform|MakeTransform (- (Transformation|GetActorLocation) "0.000000,0.000000,0.500000") (Math|Rotator|MakeRotator 0.0 0.0 0.0)) "Undefined" "MultiplyWithRoot" 0 0))