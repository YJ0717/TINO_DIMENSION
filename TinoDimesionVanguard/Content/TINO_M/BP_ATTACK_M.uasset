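; Component that gives its TINO_M_BP owner a three-hit melee combo on the IA_ATTACK input.
; Each press is gated by a busy flag, shows both weapon meshes and plays the montage for the current combo step.
; A montage notify clears the flag and advances the step, wrapping after the third attack.
; Timers started on each attack reset the combo and hide the weapons again after short delays.
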(event Custom|Reset%20COunter
  (Variables|Default|SetCBCT 0))

(event Custom|Hidden
  (Rendering|SetVisibility (Variables|Default|GetRight%20Weapon) false false))

(event Input|EnhancedActionEvents|EnhancedInputActionIA_ATTACK
  (params (ActionValue :type Boolean) (ElapsedSeconds :type Float%20%28double-precision%29) (TriggeredSeconds :type Float%20%28double-precision%29) (InputAction :type Input%20Action%20Object%20Reference :default "/Game/TINO_G/IA_TINO/IA_ATTACK.IA_ATTACK"))
  (bind _mesh (Variables|Default|GetMesh))
  (:Started
    (if (not (Variables|Default|GetAttakc?))
      (Variables|Default|SetAttakc? true)
      (Rendering|SetVisibility (Variables|Default|GetLeft%20Weapon) true false)
      (Utilities|Time|SetTimerbyEvent (delegate Custom|Hidden) 5.0)
      (switch int (Variables|Default|GetCBCT)
        (:0
          (Animation|Montage|PlayMontage _mesh "/Game/TINO_M/TINO_M_ANI/Attack_1_Montage.Attack_1_Montage"
            (:then
              (Utilities|Time|SetTimerbyEvent (delegate Custom|Reset%20COunter) 1.0 :!label _label))
            (:OnNotifyBegin
              (Variables|Default|SetAttakc? false)
              (Variables|Default|SetCBCT 1))))
        (:1
          (Animation|Montage|PlayMontage _mesh "/Game/TINO_M/TINO_M_ANI/Attack_2_Montage.Attack_2_Montage"
            (:then
              (goto _label))
            (:OnNotifyBegin
              (Variables|Default|SetAttakc? false)
              (Variables|Default|SetCBCT 2))))
        (:2
          (Animation|Montage|PlayMontage _mesh "/Game/TINO_M/TINO_M_ANI/Attack_3_Montage.Attack_3_Montage"
            (:then
              (goto _label))
            (:OnNotifyBegin
              (Variables|Default|SetAttakc? false)
              (Variables|Default|SetCBCT 0))))))))

(event EventBeginPlay
  (bind _astino_m_bp (Utilities|Casting|CastToTINO_M_BP (Components|GetOwner)))
  (bind _output_get (Variables|Default|SetTINO%20M _astino_m_bp))
  (Variables|Default|SetMesh (Variables|/Script/Engine.Character|GetMesh _output_get))
  (Variables|Default|SetLeft%20Weapon (Variables|/Game/TINO_M/TINO_M_BP.TINO_M_BP_C|GetLeft_weapon _astino_m_bp))
  (Variables|Default|SetRight%20Weapon (Variables|/Game/TINO_M/TINO_M_BP.TINO_M_BP_C|GetRight_weapon _astino_m_bp)))