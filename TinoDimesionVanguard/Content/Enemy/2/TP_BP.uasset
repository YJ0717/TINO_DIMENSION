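; TP_BP is an enemy AI character that roams, chases seen pawns and plays a melee montage that damages Player-tagged actors.
; Tick drives the chase through AIMoveTo, with IsRoaming, IsAttacking, IsFleeing and Isdead flags gating behaviors.
; A screen-projected health widget shows near the player; damage triggers hit reactions or death and destruction.
; Runaway is never called here, and the timed RegenHealth adds zero, so it restores nothing.
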(event OnSeePawn(PawnSensing)
  (params (Pawn :type Pawn%20Object%20Reference))
  ;[0.15 0.15 0.15 0.5] EventSeeingPawn
  (if (not (Variables|Default|GetIsdead))
    (Variables|Default|SetChasingPawn Pawn)))

(event Custom|Roam
  ;[0.15 0.15 0.15 0.5] roam
  (if (not (Variables|Default|GetIsdead))
    (if (not (Variables|Default|GetIsFleeing))
      (if (not (Variables|Default|GetIsRoaming))
        (if (not (Variables|Default|GetIsAttacking))
          (Variables|Default|SetIsRoaming true)
          (AI|AIMoveTo self (.RandomLocation (AI|Navigation|GetRandomReachablePointinRadius (Transformation|GetActorLocation) 1.5e+03 0 0)) 0 2.5e+02 false
            (:OnSuccess
              _)
            (:OnFail
              _))
          (Utilities|FlowControl|Delay 5.0)
          (Variables|Default|SetIsRoaming false)
          (CallFunction|Roam))))))

(event Custom|UpdatePawnChase
  ;[0.15 0.15 0.15 0.5] UpdatePawnChasing
  (Utilities|IsValid (Variables|Default|GetChasingPawn)
    (:Is%20Valid
      (if (< (Math|Vector|Distance(Vector) (Transformation|GetActorLocation (Variables|Default|GetChasingPawn)) (Transformation|GetActorLocation)) 2.5e+03)
        (if (not (Variables|Default|GetIsFleeing))
          (if (Variables|Default|GetIsdead)
            (AI|Navigation|StopMovement (AI|GetAIController self))
            (elif (not (Variables|Default|GetIsAttacking))
              (Variables|Default|SetIsAttacking true)
              (AI|Navigation|StopMovement (AI|GetAIController self))
              (AI|AIMoveTo self "0, 0, 0" (Variables|Default|GetChasingPawn) 2e+02 false
                (:OnSuccess
                  (bind _returnvalue (Animation|PlayAnimMontage "/Game/Enemy/2/TP_Animation/TP_AttackMpontage.TP_AttackMpontage" 1.0 "None"))
                  (bind _outactors (Collision|SphereOverlapActors (Transformation|GetWorldLocation (Variables|Default|GetArrow1)) 1.5e+02 (Variables|Default|GetObject%20Types) 0))
                  (bind _array_element (Utilities|Array|ForEachLoopwithBreak _outactors)
                    (:LoopBody
                      (if (Actor|ActorHasTag _array_element "Player")
                        (Game|Damage|ApplyDamage _array_element 2e+01 0 0)))
                    (:Completed
                      (Utilities|FlowControl|Delay _returnvalue)
                      (Variables|Default|SetIsAttacking false :!label _label)
                      (CallFunction|Roam))))
                (:OnFail
                  (goto _label))))))))
    (:Is%20Not%20Valid
      (CallFunction|Roam))))

(event Custom|Runaway
  (bind _returnvalue (Transformation|GetActorLocation))
  (bind _chasingpawn (Variables|Default|GetChasingPawn))
  (bind _returnvalue_2 (Transformation|GetActorLocation _chasingpawn))
  (bind _returnvalue_3 (Math|Rotator|FindLookatRotation _returnvalue _returnvalue_2))
  (bind _returnvalue_4 (Math|Vector|GetForwardVector _returnvalue_3))
  (bind _returnvalue_5 (* _returnvalue_4 -100))
  (bind _returnvalue_6 (+ _returnvalue _returnvalue_5))
  (bind (_x _y) (Math|Vector|BreakVector _returnvalue_6))
  ;[0.15 0.15 0.15 0.5] Runawway
  (if (not (Variables|Default|GetIsFleeing))
    (Variables|Default|SetIsFleeing true)
    (AI|AIMoveTo self (.RandomLocation (AI|Navigation|GetRandomReachablePointinRadius (Math|Vector|MakeVector _x _y (.Z (Math|Vector|BreakVector _returnvalue))) 5e+02 0 0)) 0 2e+02 false
      (:OnSuccess
        _)
      (:OnFail
        _))
    (Variables|Default|SetIsFleeing false)))

(event EventBeginPlay
  ;[0.15 0.15 0.15 0.5] Begin  Play
  (CallFunction|Roam)
  (Utilities|Time|SetTimerbyFunctionName 0 "RegenHealth" 1e+01 true)
  (bind _returnvalue (UserInterface|CreateWidget "/Game/Enemy/2/TP_HEALTH.TP_HEALTH_C"))
  (bind _output_get (Variables|Default|SetTP_HP_UI _returnvalue))
  (UserInterface|Viewport|AddtoViewport _output_get 0))

(event Game|Damage|EventAnyDamage
  (params (Damage :type Float%20%28single-precision%29) (DamageType :type Damage%20Type%20Object%20Reference) (InstigatedBy :type Controller%20Object%20Reference) (DamageCauser :type Actor%20Object%20Reference))
  ;[0.15 0.15 0.15 0.5] Hit_damage
  (if (not (Variables|Default|GetIsdead))
    (bind _output_get (Variables|Default|SetTPHealth (- (Variables|Default|GetTPHealth) Damage)))
    (if (> _output_get 0.01)
      (Animation|PlayAnimMontage "/Game/Enemy/2/TP_Animation/TP_Hit_Montage.TP_Hit_Montage" 1.0 "None")
      (else
        (Variables|Default|SetIsdead true)
        (Collision|SetActorEnableCollision false)
        (Components|Animation|PlayAnimation (Variables|Character|GetMesh) "/Game/Enemy/2/TP_Animation/TP_Dead.TP_Dead" false)
        (Utilities|FlowControl|Delay 5.0)
        (Actor|DestroyActor)
        (Widget|RemovefromParent (Variables|Default|GetTP_HP_UI))))))

(event EventTick
  (params (DeltaSeconds :type Float%20%28single-precision%29))
  (bind _tp_hp_ui (Variables|Default|GetTP_HP_UI))
  ;[0.15 0.15 0.15 0.5] Tick Event
  (CallFunction|UpdatePawnChase)
  (if (< (Transformation|GetDistanceTo self (Game|Player|GetPlayerPawn 0)) 1e+03)
    (Widget|SetVisibility _tp_hp_ui "Visible")
    (else
      (Widget|SetVisibility _tp_hp_ui "Hidden")))
  (Variables|Default|Setground_speed (Math|Vector|VectorLengthXY (Variables|/Script/Engine.MovementComponent|GetVelocity (Variables|Character|GetCharacterMovement))))
  (Transformation|SetWorldRotation (Variables|Default|GetArrow1) (Pawn|GetControlRotation :!class /Script/Engine.Pawn) false false)
  (Class|UserWidget|SetPositioninViewport (Variables|Default|GetTP_HP_UI) (.ScreenLocation (Class|PlayerController|ProjectWorldLocationtoScreen (Game|GetPlayerController 0) (Transformation|GetSocketLocation (Variables|Character|GetMesh) "TPHP") false)) true))

(fn ConstructionScript)

(fn RegenHealth
  (if (< (Variables|Default|GetTPHealth) 0.0)
    (Variables|Default|SetTPHealth (+ (Variables|Default|GetTPHealth) 0.0))))